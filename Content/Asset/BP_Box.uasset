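; BP_Box is a collectible pickup that the player collects with F after overlapping its box, playing a rune-collection sound.
; Overlap by player pawn 0 enables input and opens a gate, so pressing F destroys the actor; nothing here closes the gate again.
; A separate CustomEvent, not called within this graph, steps through Dialogue2 lines in a lazily created WB_Collectable widget.
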(event `Key|F`
  (params (Key :type "Key Structure"))
  (:`Pressed`
    (`/Engine/EditorBlueprintResources/StandardMacros.Gate` true :!label _label
      (:`Exit`
        (`self.K2_DestroyActor`)
        (`GameplayStatics.PlaySound2D` "/Game/Asset/SFX_CollectRunes.SFX_CollectRunes" 1.0 1.0 0.0 null null false)))))

(event `self.Box.OnComponentBeginOverlap`
  (params (OverlappedComponent :type "PrimitiveComponent Object Reference") (OtherActor :type "Actor Object Reference") (OtherComp :type "PrimitiveComponent Object Reference") (OtherBodyIndex :type Integer) (bFromSweep :type Boolean) (SweepResult :type "HitResult Structure (by ref)"))
  (if (== OtherActor (`GameplayStatics.GetPlayerPawn` 0))
    (`self.EnableInput` (`GameplayStatics.GetPlayerController` 0))
    (goto _label :!via `Open`)))

(event `CustomEvent`
  (bind _talk_index2 (`self.Talk Index2`))
  (bind _dialogue2 (`self.Dialogue2`))
  (`/Engine/EditorBlueprintResources/StandardMacros.IncrementInt` _talk_index2
    (:`  `
      (if (< _talk_index2 (`KismetArrayLibrary.Array_Length` _dialogue2))
        (`self.UI2`
          (:`then`
            _)
          (:`else`
            (bind _returnvalue (`|CreateWidget` "/Game/Collectable/WB_Collectable.WB_Collectable_C" (`GameplayStatics.GetPlayerController` 0)))
            (bind _output_get (set `self.UI2` _returnvalue))
            (`UserWidget.AddToViewport` _output_get 0)))
        (`TextBlock.SetText` (`/Game/Collectable/WB_Collectable.TalkText2` (`self.UI2`)) (`KismetTextLibrary.Conv_StringToText` (`|GetArrayItem` _dialogue2 _talk_index2)))))))

(fn `UserConstructionScript`)