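; Behavior tree task that makes the boss either attack player 0 or turn toward them.
; It updates the "Player" motion warping target, then uses rounded forward and right dot products to choose.
; A player clearly to the side triggers a turn montage, then the capsule snaps to face them.
; Otherwise, including directly behind, distance picks a random short- or long-range attack montage at a random play rate.
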(event `self.ReceiveExecuteAI`
  (params (OwnerController :type "AIController Object Reference") (ControlledPawn :type "Pawn Object Reference"))
  (bind _returnvalue (`KismetMathLibrary.RandomFloatInRange` 1.0 2.0))
  (bind _asbp_boss (cast `/Game/Yuqi/AI_Boss/BP_Boss` ControlledPawn)
    (:`then`
      (bind _returnvalue_2 (- (`Actor.K2_GetActorLocation` (`GameplayStatics.GetPlayerPawn` 0)) (`Actor.K2_GetActorLocation` _asbp_boss)))
      (set `self.intermediate_distance` (`KismetMathLibrary.VSize` _returnvalue_2))
      (`MotionWarpingComponent.AddOrUpdateWarpTargetFromTransform` (`/Game/Yuqi/AI_Boss/BP_Boss.MotionWarping` _asbp_boss) "Player" (`Actor.GetTransform` (`GameplayStatics.GetPlayerPawn` 0)))
      (bind _returnvalue_3 (`KismetMathLibrary.Normal` _returnvalue_2))
      (set `self.ToTarget` _returnvalue_3)
      (bind _capsulecomponent (`Character.CapsuleComponent` _asbp_boss))
      (switch `int` (`KismetMathLibrary.Round` (`KismetMathLibrary.Dot_VectorVector` (`KismetMathLibrary.Normal` (`SceneComponent.GetForwardVector` _capsulecomponent)) _returnvalue_3))
        (:`Default`
          (if (<= (`self.intermediate_distance`) 2000.0) :!label _label
            (bind _mesh (`Character.Mesh` _asbp_boss))
            (`|PlayMontage` _mesh (`KismetArrayLibrary.Array_Random` (`self.Montage to Play_Short`)) (`KismetMathLibrary.RandomFloatInRange` 0.5 0.85)
              (:`OnCompleted`
                (`self.FinishExecute` true :!label _label_2))
              (:`OnInterrupted`
                (`self.FinishExecute` false :!label _label_3)))
            (else
              (`|PlayMontage` _mesh (`KismetArrayLibrary.Array_Random` (`self.Montage to Play_Long`)) (`KismetMathLibrary.RandomFloatInRange` 0.3 0.5)
                (:`OnCompleted`
                  (goto _label_2))
                (:`OnInterrupted`
                  (goto _label_3))))))
        (:`-1`
          (switch `int` (`KismetMathLibrary.Round` (`KismetMathLibrary.Dot_VectorVector` (`KismetMathLibrary.Normal` (`SceneComponent.GetRightVector` _capsulecomponent)) (`self.ToTarget`))) :!label _label_4
            (:`Default`
              (goto _label))
            (:`-1`
              (`|PlayMontage` _mesh "/Game/Yuqi/AI_Boss/Animations/IdleTurnLeft_Montage.IdleTurnLeft_Montage" _returnvalue
                (:`OnCompleted`
                  (`SceneComponent.K2_SetWorldRotation` _capsulecomponent (`KismetMathLibrary.Conv_VectorToRotator` (`self.ToTarget`)) false false :!label _label_5)
                  (`self.FinishExecute` true))
                (:`OnInterrupted`
                  (`self.FinishExecute` false :!label _label_6))))
            (:`0`
              (goto _label))
            (:`1`
              (`|PlayMontage` _mesh "/Game/Yuqi/AI_Boss/Animations/IdleTurnRight_Montage.IdleTurnRight_Montage" _returnvalue
                (:`OnCompleted`
                  (goto _label_5))
                (:`OnInterrupted`
                  (goto _label_6))))))
        (:`0`
          (goto _label_4))
        (:`1`
          (goto _label))))
    (:`CastFailed`
      (`self.FinishExecute` false))))