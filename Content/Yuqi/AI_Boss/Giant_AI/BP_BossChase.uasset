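; Behavior tree task that makes the giant boss chase the player or, when a lure is active, go for the lure.
; Without a lure it runs AI MoveTo on the player with a randomized acceptance radius.
; With one, it targets the blackboard's sand NPC dummy; the computed point away from it is overridden by Target Actor.
; Move results finish the task, but a failed lure cast never does.
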(event `self.ReceiveExecuteAI`
  (params (OwnerController :type "AIController Object Reference") (ControlledPawn :type "Pawn Object Reference"))
  (bind _returnvalue (`GameplayStatics.GetPlayerPawn` 0))
  (bind _returnvalue_2 (`AIBlueprintHelperLibrary.GetBlackboard` OwnerController))
  (if (not (`BlackboardComponent.GetValueAsBool` _returnvalue_2 (`self.Key_HasLure`)))
    (`|AIMoveTo` ControlledPawn (`Actor.K2_GetActorLocation` _returnvalue) _returnvalue (`KismetMathLibrary.RandomFloatInRange` 15.0 300.0)
      (:`OnSuccess`
        (`self.FinishExecute` true :!label _label))
      (:`OnFail`
        (`self.FinishExecute` false :!label _label_2)))
    (else
      (bind _asbp_sand_npcdummy (cast `/Game/Yuqi/Blueprint/BP_SandNPCDummy` (`BlackboardComponent.GetValueAsObject` _returnvalue_2 (`self.Key_LureObject`))))
      (bind _returnvalue_3 (`SceneComponent.K2_GetComponentLocation` (`/Game/Yuqi/Blueprint/BP_SandNPCDummy.DefaultSceneRoot` _asbp_sand_npcdummy)))
      (`|AIMoveTo` ControlledPawn (+ _returnvalue_3 (* (- (`Actor.K2_GetActorLocation` ControlledPawn) _returnvalue_3) 1000)) _asbp_sand_npcdummy
        (:`OnSuccess`
          (goto _label))
        (:`OnFail`
          (goto _label_2))))))