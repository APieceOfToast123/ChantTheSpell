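; BP_BossAttack is a Behavior Tree task that makes the giant boss (BP_Boss) play an attack montage.
; It measures the distance to player 0 and picks a random montage from the short-range set within 2000 units, otherwise from the long-range set.
; The montage plays at reduced speed, and the task succeeds on completion or fails on interruption or a failed boss cast.
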(event `self.ReceiveExecuteAI`
  (params (OwnerController :type "AIController Object Reference") (ControlledPawn :type "Pawn Object Reference"))
  (bind _asbp_boss (cast `/Game/Yuqi/AI_Boss/BP_Boss` ControlledPawn)
    (:`then`
      (set `self.intermediate_distance` (`KismetMathLibrary.VSize` (- (`Actor.K2_GetActorLocation` _asbp_boss) (`Actor.K2_GetActorLocation` (`GameplayStatics.GetPlayerPawn` 0)))))
      (if (<= (`self.intermediate_distance`) 2000.0)
        (bind _mesh (`Character.Mesh` _asbp_boss))
        (`|PlayMontage` _mesh (`KismetArrayLibrary.Array_Random` (`self.Montage to Play_Short`)) 0.3
          (:`OnCompleted`
            (`self.FinishExecute` true :!label _label))
          (:`OnInterrupted`
            (`self.FinishExecute` false :!label _label_2)))
        (else
          (`|PlayMontage` _mesh (`KismetArrayLibrary.Array_Random` (`self.Montage to Play_Long`)) 0.3
            (:`OnCompleted`
              (goto _label))
            (:`OnInterrupted`
              (goto _label_2))))))
    (:`CastFailed`
      (goto _label_2))))