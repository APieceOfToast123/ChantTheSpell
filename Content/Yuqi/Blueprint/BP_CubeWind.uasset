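; Box-shaped wind tunnel that pushes physics bodies and the player character along the actor's up vector.
; Construction script sizes the overlap box and WindZone from tunnel width and height.
; Each tick, a grid of line traces applies force at hit points on physics bodies and, while the zone is occupied, launches the character.
; Entering cancels gliding and sets gravity and air control; leaving marks jumping and rechecks gliding.
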(event `Blow Physics Items`
  (bind _returnvalue (`self.GetTransform`))
  (bind _wind_tunnel_width (`self.Wind Tunnel Width`))
  (bind _distance_between_line_trace (`self.Distance Between Line Trace`))
  (bind _returnvalue_2 (`KismetMathLibrary.FTrunc` (/ (* (`self.Wind Tunnel Width`) 2.0) (`self.Distance Between Line Trace`))))
  (for _index (range (+ _returnvalue_2 1))
    (for _index_2 (range (+ _returnvalue_2 1))
      (bind _returnvalue_3 (`KismetMathLibrary.MakeVector` (- _wind_tunnel_width (* _index_2 _distance_between_line_trace)) (- _wind_tunnel_width (* _index _distance_between_line_trace))))
      (bind (_outhit _returnvalue_4) (`KismetSystemLibrary.LineTraceSingleForObjects` (- (`KismetMathLibrary.TransformLocation` _returnvalue _returnvalue_3) (0.0 0.0 600.0)) (- (`KismetMathLibrary.TransformLocation` _returnvalue (+ _returnvalue_3 (`KismetMathLibrary.MakeVector` 0.0 0.0 (* (`self.Wind Tunnel Height`) 1.5)))) (0.0 0.0 200.0)) (`|MakeArray` "ObjectTypeQuery4" :!type "EObjectTypeQuery Enum")))
      (if _returnvalue_4
        (bind (_bblockinghit _binitialoverlap _time _distance _location _impactpoint _normal _impactnormal _physmat _hitactor _hitcomponent) (`GameplayStatics.BreakHitResult` _outhit))
        (`PrimitiveComponent.AddForceAtLocation` _hitcomponent (* (`self.GetActorUpVector`) (`self.Wind Force`)) _impactpoint "None")))))

(event `self.Box Wind Range.OnComponentBeginOverlap`
  (params (OverlappedComponent :type "PrimitiveComponent Object Reference") (OtherActor :type "Actor Object Reference") (OtherComp :type "PrimitiveComponent Object Reference") (OtherBodyIndex :type Integer) (bFromSweep :type Boolean) (SweepResult :type "HitResult Structure (by ref)"))
  (bind _charactermovement (`Character.CharacterMovement` (`self.PlayerREF`)))
  (set `self.Is In Wind Zone` true)
  (bind _asbp_third_person_character_1 (cast `/Game/ThirdPerson/Blueprints/BP_ThirdPersonCharacter1` OtherActor))
  (bind _output_get (set `self.PlayerREF` _asbp_third_person_character_1))
  ; 没有收降落伞动作的收降落伞(取消滑翔模拟)
  (set `/Game/ThirdPerson/Blueprints/BP_ThirdPersonCharacter1.State_isGliding` false _output_get)
  (set `/Game/ThirdPerson/Blueprints/BP_ThirdPersonCharacter1.State_isJumping` false _output_get)
  (set `CharacterMovementComponent.GravityScale` 1.75 _charactermovement)
  (set `CharacterMovementComponent.AirControl` 0.35 _charactermovement))

(event `self.Box Wind Range.OnComponentEndOverlap`
  (params (OverlappedComponent :type "PrimitiveComponent Object Reference") (OtherActor :type "Actor Object Reference") (OtherComp :type "PrimitiveComponent Object Reference") (OtherBodyIndex :type Integer))
  (set `self.Is In Wind Zone` false)
  (bind _asbp_third_person_character_1 (cast `/Game/ThirdPerson/Blueprints/BP_ThirdPersonCharacter1` OtherActor))
  (bind _output_get (set `self.PlayerREF` _asbp_third_person_character_1))
  (set `/Game/ThirdPerson/Blueprints/BP_ThirdPersonCharacter1.State_isJumping` true _output_get)
  (set `/Game/ThirdPerson/Blueprints/BP_ThirdPersonCharacter1.State_isJumping` true _output_get)
  (`/Game/ThirdPerson/Blueprints/BP_ThirdPersonCharacter1.Check can Glide` _output_get))

(event `self.ReceiveTick`
  (params (DeltaSeconds :type "Float (single-precision)"))
  (`self.Blow Physics Items`)
  (if (`self.Is In Wind Zone`)
    (`self.Blow Pawn`)))

(event `Blow Pawn`
  (bind _returnvalue (`self.GetTransform`))
  (bind (_returnvalue_location _returnvalue_rotation) (`KismetMathLibrary.BreakTransform` (`self.GetTransform`)))
  (bind _wind_tunnel_width (`self.Wind Tunnel Width`))
  (bind _distance_between_line_trace (`self.Distance Between Line Trace`))
  (bind _returnvalue_2 (`KismetMathLibrary.FTrunc` (/ (* (`self.Wind Tunnel Width`) 2.0) (`self.Distance Between Line Trace`))))
  (for _index (range (+ _returnvalue_2 1))
    (for _index_2 (range (+ _returnvalue_2 1))
      (bind _returnvalue_3 (`KismetMathLibrary.MakeVector` (- _wind_tunnel_width (* _index_2 _distance_between_line_trace)) (- _wind_tunnel_width (* _index _distance_between_line_trace))))
      (bind (_outhit _returnvalue_4) (`KismetSystemLibrary.LineTraceSingleForObjects` :`Start` (- (`KismetMathLibrary.TransformLocation` _returnvalue _returnvalue_3) (0.0 0.0 600.0)) :`End` (- (`KismetMathLibrary.TransformLocation` _returnvalue (+ _returnvalue_3 (`KismetMathLibrary.MakeVector` 0.0 0.0 (* (`self.Wind Tunnel Height`) 2.0)))) (0.0 0.0 200.0)) :`ObjectTypes` (`|MakeArray` "ObjectTypeQuery3" :!type "EObjectTypeQuery Enum") :`TraceColor` (struct :`R` 1.0 :`G` 0.804551 :`B` 0.05872 :`A` 1.0) :`TraceHitColor` (struct :`R` 1.0 :`B` 0.590601 :`A` 1.0)))
      (if _returnvalue_4
        (bind _asbp_third_person_character_1 (cast `/Game/ThirdPerson/Blueprints/BP_ThirdPersonCharacter1` (`.HitActor` (`GameplayStatics.BreakHitResult` _outhit))))
        (set `self.PlayerREF` _asbp_third_person_character_1)
        (`Character.LaunchCharacter` (`self.PlayerREF`) (* (`KismetMathLibrary.GetUpVector` _returnvalue_rotation) (* (`self.Wind Force`) (`self.PawnOffset`))) false true)))))

(fn `UserConstructionScript`
  (bind _wind_tunnel_width (`self.Wind Tunnel Width`))
  (bind _returnvalue (/ (`self.Wind Tunnel Width`) 50.0))
  (`BoxComponent.SetBoxExtent` (`self.Box Wind Range`) (`KismetMathLibrary.MakeVector` _wind_tunnel_width _wind_tunnel_width (`self.Wind Tunnel Height`)) true)
  (`SceneComponent.SetRelativeScale3D` (`self.Wind Zone`) (`KismetMathLibrary.MakeVector` _returnvalue _returnvalue (/ (`self.Wind Tunnel Height`) 50.0))))