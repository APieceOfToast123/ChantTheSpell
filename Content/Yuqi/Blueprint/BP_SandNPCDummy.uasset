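; Liftable cube dummy actor that shows a "Click B to Lift Cube" prompt widget when the player character is nearby.
; Tick toggles the prompt by distance, turns it toward the player's follow camera and keeps it above the mesh along its up vector.
; HandleLift flips and returns IsLifted and toggles the prompt, but does no movement itself.
; Tick ignores IsLifted, so it overrides that visibility change.
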(event `self.ReceiveBeginPlay`
  (bind _aswb_press_to_do (cast `/Game/Yuqi/UI/WB_PressToDo` (`WidgetComponent.GetWidget` (`self.Widget`))))
  (set `TextBlock.Text` "Click B to Lift Cube" (`/Game/Yuqi/UI/WB_PressToDo.Text` _aswb_press_to_do)))

(event `self.ReceiveTick`
  (params (DeltaSeconds :type "Float (single-precision)"))
  (bind _staticmesh (`self.StaticMesh`))
  (bind _widget (`self.Widget`))
  (bind _asbp_third_person_character_1 (cast `/Game/ThirdPerson/Blueprints/BP_ThirdPersonCharacter1` (`GameplayStatics.GetPlayerCharacter` 0)))
  (if (< (`KismetMathLibrary.Abs` (`KismetMathLibrary.Vector_Distance` (`self.K2_GetActorLocation` _asbp_third_person_character_1) (`self.K2_GetActorLocation`))) 500.0)
    (`SceneComponent.SetVisibility` (`self.Widget`) true false)
    (`SceneComponent.K2_SetWorldRotation` _widget (`KismetMathLibrary.FindLookAtRotation` (`SceneComponent.K2_GetComponentLocation` _widget) (`SceneComponent.K2_GetComponentLocation` (`/Game/ThirdPerson/Blueprints/BP_ThirdPersonCharacter1.FollowCamera` _asbp_third_person_character_1))) false false)
    (`SceneComponent.K2_SetWorldLocation` (`self.Widget`) (+ (`SceneComponent.K2_GetComponentLocation` _staticmesh) (* (`KismetMathLibrary.GetUpVector` (`SceneComponent.K2_GetComponentRotation` _staticmesh)) 170)) false false)
    (else
      (`SceneComponent.SetVisibility` (`self.Widget`) false false))))

(fn `HandleLift`
  (returns (`isLiftedVaild?` :type Boolean))
  (if (`self.isLifted?`)
    (set `self.isLifted?` false)
    (`SceneComponent.SetVisibility` (`self.Widget`) true false)
    (else
      (set `self.isLifted?` true)
      (`SceneComponent.SetVisibility` (`self.Widget`) false false)))
  (return (`self.isLifted?`)))

(fn `UserConstructionScript`)