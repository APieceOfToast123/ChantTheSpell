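; BP_SequencerTrigger is a one-shot trigger volume that plays a cutscene when the player walks into it.
; Box overlap casts to BP_ThirdPersonCharacter1, stores the reference and plays the referenced Level Sequence.
; It disables the character's movement shortly after, restores walking after a fixed delay, then destroys itself.
; The freeze relies on hardcoded delays rather than the sequence's finished event.
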(event `self.Box.OnComponentBeginOverlap`
  (params (OverlappedComponent :type "PrimitiveComponent Object Reference") (OtherActor :type "Actor Object Reference") (OtherComp :type "PrimitiveComponent Object Reference") (OtherBodyIndex :type Integer) (bFromSweep :type Boolean) (SweepResult :type "HitResult Structure (by ref)"))
  (bind _asbp_third_person_character_1 (cast `/Game/ThirdPerson/Blueprints/BP_ThirdPersonCharacter1` OtherActor))
  (set `self.PlayerREF` _asbp_third_person_character_1)
  (`MovieSceneSequencePlayer.Play` (`LevelSequenceActor.SequencePlayer` (`self.Level Sequencer`)))
  (`KismetSystemLibrary.Delay` 0.5)
  (`CharacterMovementComponent.SetMovementMode` (`Character.CharacterMovement` (`self.PlayerREF`)) "MOVE_None" 0)
  (`KismetSystemLibrary.Delay` 10.0)
  (`CharacterMovementComponent.SetMovementMode` (`Character.CharacterMovement` (`self.PlayerREF`)) "MOVE_Walking" 0)
  (`self.K2_DestroyActor`))

(fn `UserConstructionScript`)