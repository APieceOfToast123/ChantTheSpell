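; Wind tunnel actor that pushes physics objects and the third-person character along its up axis, sized by the construction script from tunnel radius and height.
; Every tick, a grid of line traces applies force at physics-body hit points and, while the zone is overlapped, launches the character.
; Entering cancels gliding and sets gravity and air control; leaving re-checks gliding, with a counter-launch if the tunnel is rotated.
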(event `Blow Physics Items`
  (bind _returnvalue (`self.GetTransform`))
  (bind _distance_between_line_trace (`self.Distance Between Line Trace`))
  (bind _returnvalue_2 (`CapsuleComponent.GetScaledCapsuleRadius` (`self.Wind Range`)))
  (bind _returnvalue_3 (`KismetMathLibrary.FTrunc` (/ (* (`CapsuleComponent.GetScaledCapsuleRadius` (`self.Wind Range`)) 2.0) (`self.Distance Between Line Trace`))))
  (for _index (range (+ _returnvalue_3 1))
    (for _index_2 (range (+ _returnvalue_3 1))
      (bind _returnvalue_4 (`KismetMathLibrary.MakeVector` (- _returnvalue_2 (* _index_2 _distance_between_line_trace)) (- _returnvalue_2 (* _index _distance_between_line_trace))))
      (bind (_outhit _returnvalue_5) (`KismetSystemLibrary.LineTraceSingleForObjects` (`KismetMathLibrary.TransformLocation` _returnvalue _returnvalue_4) (`KismetMathLibrary.TransformLocation` _returnvalue (+ _returnvalue_4 (`KismetMathLibrary.MakeVector` 0.0 0.0 (* (`CapsuleComponent.CapsuleHalfHeight` (`self.Wind Range`)) 1.5)))) (`|MakeArray` "ObjectTypeQuery4" :!type "EObjectTypeQuery Enum")))
      (if _returnvalue_5
        (bind (_bblockinghit _binitialoverlap _time _distance _location _impactpoint _normal _impactnormal _physmat _hitactor _hitcomponent) (`GameplayStatics.BreakHitResult` _outhit))
        (`PrimitiveComponent.AddForceAtLocation` _hitcomponent (* (`self.GetActorUpVector`) (`self.Wind Force`)) _impactpoint "None")))))

(event `self.Wind Range.OnComponentBeginOverlap`
  (params (OverlappedComponent :type "PrimitiveComponent Object Reference") (OtherActor :type "Actor Object Reference") (OtherComp :type "PrimitiveComponent Object Reference") (OtherBodyIndex :type Integer) (bFromSweep :type Boolean) (SweepResult :type "HitResult Structure (by ref)"))
  (bind _charactermovement (`Character.CharacterMovement` (`self.PlayerREF`)))
  (set `self.Is In Wind Zone` true)
  (bind _asbp_third_person_character (cast `/Game/ThirdPerson/Blueprints/BP_ThirdPersonCharacter` OtherActor))
  (bind _output_get (set `self.PlayerREF` _asbp_third_person_character))
  ; 没有收降落伞动作的收降落伞(取消滑翔模拟)
  (set `/Game/ThirdPerson/Blueprints/BP_ThirdPersonCharacter.State_isGliding` false _output_get)
  (set `/Game/ThirdPerson/Blueprints/BP_ThirdPersonCharacter.State_isJumping` false _output_get)
  (set `CharacterMovementComponent.GravityScale` 1.75 _charactermovement)
  (set `CharacterMovementComponent.AirControl` 0.35 _charactermovement))

(event `self.Wind Range.OnComponentEndOverlap`
  (params (OverlappedComponent :type "PrimitiveComponent Object Reference") (OtherActor :type "Actor Object Reference") (OtherComp :type "PrimitiveComponent Object Reference") (OtherBodyIndex :type Integer))
  (bind (_returnvalue_location _returnvalue_rotation) (`KismetMathLibrary.BreakTransform` (`self.GetTransform`)))
  (set `self.Is In Wind Zone` false)
  (bind _asbp_third_person_character (cast `/Game/ThirdPerson/Blueprints/BP_ThirdPersonCharacter` OtherActor))
  (bind _output_get (set `self.PlayerREF` _asbp_third_person_character))
  (set `/Game/ThirdPerson/Blueprints/BP_ThirdPersonCharacter.State_isJumping` true _output_get)
  (`/Game/ThirdPerson/Blueprints/BP_ThirdPersonCharacter.Check can Glide` _output_get)
  (if (!= (`self.K2_GetActorRotation`) (struct))
    (`Character.LaunchCharacter` (`self.PlayerREF`) (* (* (`KismetMathLibrary.GetUpVector` _returnvalue_rotation) (* (`self.Wind Force`) (`self.Pawn Lose Weight Offset`))) -0.3) false true)))

(event `self.ReceiveTick`
  (params (DeltaSeconds :type "Float (single-precision)"))
  (`self.Blow Physics Items`)
  (if (`self.Is In Wind Zone`)
    (`self.Blow Pawn`)))

(event `Blow Pawn`
  (bind _returnvalue (`self.GetTransform`))
  (bind (_returnvalue_location _returnvalue_rotation) (`KismetMathLibrary.BreakTransform` (`self.GetTransform`)))
  (bind _distance_between_line_trace (`self.Distance Between Line Trace`))
  (bind _returnvalue_2 (`CapsuleComponent.GetScaledCapsuleRadius` (`self.Wind Range`)))
  (bind _returnvalue_3 (`KismetMathLibrary.FTrunc` (/ (* (`CapsuleComponent.GetScaledCapsuleRadius` (`self.Wind Range`)) 2.0) (`self.Distance Between Line Trace`))))
  (for _index (range (+ _returnvalue_3 1))
    (for _index_2 (range (+ _returnvalue_3 1))
      (bind _returnvalue_4 (`KismetMathLibrary.MakeVector` (- _returnvalue_2 (* _index_2 _distance_between_line_trace)) (- _returnvalue_2 (* _index _distance_between_line_trace))))
      (bind (_outhit _returnvalue_5) (`KismetSystemLibrary.LineTraceSingleForObjects` :`Start` (- (`KismetMathLibrary.TransformLocation` _returnvalue _returnvalue_4) (0.0 0.0 100.0)) :`End` (`KismetMathLibrary.TransformLocation` _returnvalue (+ _returnvalue_4 (`KismetMathLibrary.MakeVector` 0.0 0.0 (* (`CapsuleComponent.CapsuleHalfHeight` (`self.Wind Range`)) 2.0)))) :`ObjectTypes` (`|MakeArray` "ObjectTypeQuery3" :!type "EObjectTypeQuery Enum") :`TraceColor` (struct :`R` 1.0 :`G` 0.804551 :`B` 0.05872 :`A` 1.0) :`TraceHitColor` (struct :`R` 1.0 :`B` 0.590601 :`A` 1.0)))
      (if _returnvalue_5
        (bind _asbp_third_person_character (cast `/Game/ThirdPerson/Blueprints/BP_ThirdPersonCharacter` (`.HitActor` (`GameplayStatics.BreakHitResult` _outhit))))
        (set `self.PlayerREF` _asbp_third_person_character)
        (`Character.LaunchCharacter` (`self.PlayerREF`) (* (`KismetMathLibrary.GetUpVector` _returnvalue_rotation) (* (`self.Wind Force`) (`self.Pawn Lose Weight Offset`))) false true)))))

(fn `UserConstructionScript`
  (bind _wind_range (`self.Wind Range`))
  (bind _returnvalue (/ (`self.Wind Tunnel Radius`) 50.0))
  (`CapsuleComponent.SetCapsuleHalfHeight` _wind_range (`self.Wind Tunnel Height`) true)
  (`CapsuleComponent.SetCapsuleRadius` _wind_range (`self.Wind Tunnel Radius`) true)
  (`SceneComponent.SetRelativeScale3D` (`self.Wind Zone`) (`KismetMathLibrary.MakeVector` _returnvalue _returnvalue (/ (`self.Wind Tunnel Height`) 50.0))))