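; BP_SandAnchor is a pair of anchor blocks with a sand bridge between them that can be built and broken.
; The construction script sizes the range box, anchors and bridge from length, width and height variables, with SeeBridge choosing whether it starts built.
; BuildASandBridge plays Niagara and sound, then reveals a solid bridge after a delay.
; BreakSandBridge hides it with breakdown effects, and flags track the build/break state.
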(event `Build A Sand Bridge`
  (bind _sandbridge (`self.SandBridge`))
  (if (`self.canBuildBridge`)
    (set `self.canBuildBridge` false)
    (`ActorComponent.Activate` (`self.Niagara`) false)
    (`GameplayStatics.PlaySound2D` "/Game/Qianlin/Asset/SFX_Success.SFX_Success" 1.0 1.0 0.0 null null)
    (`KismetSystemLibrary.Delay` 5.0)
    (`SceneComponent.SetVisibility` _sandbridge true false)
    (`PrimitiveComponent.SetCollisionEnabled` _sandbridge "QueryAndPhysics")
    (set `self.canBreak?` true)))

(event `Break Sand Bridge`
  (bind _sandbridge (`self.SandBridge`))
  (`SceneComponent.SetVisibility` _sandbridge false false)
  (`PrimitiveComponent.SetCollisionEnabled` _sandbridge "NoCollision")
  (`ActorComponent.Activate` (`self.NS_SandBreakDown`) false)
  (`GameplayStatics.PlaySound2D` "/Game/Qianlin/Asset/SFX_Success.SFX_Success" 1.0 1.0 0.0 null null)
  (`KismetSystemLibrary.Delay` 0.7)
  (set `self.canBreak?` false)
  (set `self.canBuildBridge` true))

(fn `UserConstructionScript`
  (bind _cubeend (`self.CubeEnd`))
  (bind _sandbridge (`self.SandBridge`))
  (bind _cubestart (`self.CubeStart`))
  (`BoxComponent.SetBoxExtent` (`self.Box Range`) (`KismetMathLibrary.MakeVector` (`self.Bridge Length`) (`self.Anchor Width Y`) (`self.Anchor Height Z`)) true)
  (`SceneComponent.SetRelativeScale3D` _cubestart (`KismetMathLibrary.MakeVector` (/ (`self.Anchor Length X`) 50.0) (/ (`self.Anchor Width Y`) 50.0) (/ (`self.Anchor Height Z`) 50.0)))
  (`SceneComponent.K2_SetRelativeLocation` _cubestart (`KismetMathLibrary.MakeVector` (- (* (`self.Bridge Length`) -1.0) (`self.Anchor Length X`))) false false)
  (`SceneComponent.SetRelativeScale3D` _cubeend (`KismetMathLibrary.MakeVector` (/ (`self.Anchor Length X`) 50.0) (/ (`self.Anchor Width Y`) 50.0) (/ (`self.Anchor Height Z`) 50.0)))
  (`SceneComponent.K2_SetRelativeLocation` _cubeend (`KismetMathLibrary.MakeVector` (+ (`self.Bridge Length`) (`self.Anchor Length X`))) false false)
  (`SceneComponent.SetRelativeScale3D` _sandbridge (`KismetMathLibrary.MakeVector` (/ (`self.Bridge Length`) 50.0) (/ (`self.Anchor Width Y`) 50.0) (/ (`self.Anchor Height Z`) 50.0)))
  (if (`self.SeeBridge?`)
    (`SceneComponent.SetVisibility` _sandbridge true false)
    (`PrimitiveComponent.SetCollisionEnabled` _sandbridge "QueryAndPhysics")
    (set `self.canBreak?` true)
    (set `self.canBuildBridge` false)
    (else
      (`SceneComponent.SetVisibility` _sandbridge false false)
      (`PrimitiveComponent.SetCollisionEnabled` _sandbridge "NoCollision"))))