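; Readable paper note that shows a paper image and optional dialogue when the player interacts nearby.
; Box overlap toggles the prompt and a gate on IA_Interact, which fires Talk.
; Talk steps through DialogueList in WB_Dialogue using an index with -1 as the closing state, or flip-flops the image when the list is empty.
; Reading disables character movement, and CallEReading fires on opening and closing.
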(event `self.ReceiveBeginPlay`
  (bind _aswb_press_to_do (cast `/Game/Yuqi/UI/WB_PressToDo` (`WidgetComponent.GetWidget` (`self.Widget`))))
  (bind _output_get (set `self.Guide Text` (`/Game/Yuqi/UI/WB_PressToDo.Text` _aswb_press_to_do)))
  (`TextBlock.SetOpacity` _output_get 0.0))

(event `EnhancedInput|/Game/ThirdPerson/Input/Actions/IA_Interact`
  (params (ActionValue :type Boolean) (ElapsedSeconds :type "Float (double-precision)") (TriggeredSeconds :type "Float (double-precision)") (InputAction :type "InputAction Object Reference" :default "/Game/ThirdPerson/Input/Actions/IA_Interact.IA_Interact"))
  (:`Triggered`
    (`/Engine/EditorBlueprintResources/StandardMacros.Gate` true :!label _label
      (:`Exit`
        (`/Game/Dialogue/BPI_Dialogue.Talk`)))))

(event `self.Box.OnComponentBeginOverlap`
  (params (OverlappedComponent :type "PrimitiveComponent Object Reference") (OtherActor :type "Actor Object Reference") (OtherComp :type "PrimitiveComponent Object Reference") (OtherBodyIndex :type Integer) (bFromSweep :type Boolean) (SweepResult :type "HitResult Structure (by ref)"))
  (if (== OtherActor (`GameplayStatics.GetPlayerPawn` 0))
    (`TextBlock.SetOpacity` (`self.Guide Text`) 1.0)
    (`self.EnableInput` (`GameplayStatics.GetPlayerController` 0))
    (goto _label :!via `Open`)))

(event `self.Box.OnComponentEndOverlap`
  (params (OverlappedComponent :type "PrimitiveComponent Object Reference") (OtherActor :type "Actor Object Reference") (OtherComp :type "PrimitiveComponent Object Reference") (OtherBodyIndex :type Integer))
  (`TextBlock.SetOpacity` (`self.Guide Text`) 0.0)
  (`self.Hide Paper Image`)
  (goto _label :!via `Close`))

(event `self.Talk`
  (if (!= (`KismetArrayLibrary.Array_Length` (`self.Dialogue List`)) 0)
    (switch `int` (`self.PointerNextText`)
      (:`Default`
        (`TextBlock.SetText` (`/Game/Dialogue/WB_Dialogue.TalkText` (`self.UIBox_REF`)) (`|GetArrayItem` (`self.Dialogue List`) (`self.PointerNextText`)) :!label _label_2)
        (`TextBlock.SetOpacity` (`self.Guide Text`) 0.0)
        (`/Engine/EditorBlueprintResources/StandardMacros.IncrementInt` (`self.PointerNextText`)
          (:`  `
            (if (== (`self.PointerNextText`) (`KismetArrayLibrary.Array_Length` (`self.Dialogue List`)))
              (set `self.PointerNextText` -1)))))
      (:`-1`
        (`Widget.RemoveFromParent` (`self.UIBox_REF`))
        (`/Engine/EditorBlueprintResources/StandardMacros.IncrementInt` (`self.PointerNextText`)
          (:`  `
            (`CharacterMovementComponent.SetMovementMode` (`Character.CharacterMovement` (`GameplayStatics.GetPlayerCharacter` 0)) "MOVE_Walking" 0)
            (`TextBlock.SetOpacity` (`self.Guide Text`) 1.0)
            (`self.Hide Paper Image`)
            (`self.E_Reading`))))
      (:`0`
        (`self.E_Reading`)
        (`self.Show Paper Image`)
        (bind _returnvalue (`|CreateWidget` "/Game/Dialogue/WB_Dialogue.WB_Dialogue_C"))
        (bind _output_get (set `self.UIBox_REF` _returnvalue))
        (`UserWidget.AddToViewport` _output_get 0)
        (`CharacterMovementComponent.SetMovementMode` (`Character.CharacterMovement` (`GameplayStatics.GetPlayerCharacter` 0)) "MOVE_None" 0)
        (goto _label_2)))
    (else
      (`/Engine/EditorBlueprintResources/StandardMacros.FlipFlop`
        (:`A`
          (`self.Show Paper Image`)
          (`CharacterMovementComponent.SetMovementMode` (`Character.CharacterMovement` (`GameplayStatics.GetPlayerCharacter` 0)) "MOVE_None" 0)
          (`self.E_Reading`))
        (:`B`
          (`self.Hide Paper Image`)
          (`CharacterMovementComponent.SetMovementMode` (`Character.CharacterMovement` (`GameplayStatics.GetPlayerCharacter` 0)) "MOVE_Walking" 0)
          (`self.E_Reading`))))))

(event `Show Paper Image`
  (if (!= (`self.PaperImage`) null)
    (bind _returnvalue (`|CreateWidget` "/Game/Yuqi/UI/WB_PaperNotes.WB_PaperNotes_C"))
    (bind _output_get (set `self.UIPaper_REF` _returnvalue))
    (`Image.SetBrushFromTexture` (`/Game/Yuqi/UI/WB_PaperNotes.Image` _output_get) (`self.PaperImage`) true)
    (`UserWidget.AddToViewport` (`self.UIPaper_REF`) 0)
    (else
      (`KismetSystemLibrary.PrintString` "Didn't assign paper picture"))))

(event `Hide Paper Image`
  (if (!= (`self.UIPaper_REF`) null)
    (`Widget.RemoveFromParent` (`self.UIPaper_REF`))))

(fn `UserConstructionScript`)