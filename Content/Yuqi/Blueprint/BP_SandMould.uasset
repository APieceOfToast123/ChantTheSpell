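; BP_SandMould is a mould actor that produces a BP_SandCube on demand, keeping one cube at a time.
; Moulding, gated by CanMouldCube, destroys the previous cube, activates Niagara, waits, then spawns a new cube at the mould's transform.
; CubeMove then uses a Timeline to slide TransparentCube along the actor's forward vector, reverses it, and re-enables moulding after a short delay.
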(event `Moulding`
  (if (`self.canMouldCube?`)
    (set `self.canMouldCube?` false)
    (if (!= (`self.AlreadyMouldActor`) null)
      (`self.K2_DestroyActor` (`self.AlreadyMouldActor`)))
    (`ActorComponent.Activate` (`self.Niagara`) false)
    (`KismetSystemLibrary.Delay` 5.0)
    (bind _returnvalue (`|SpawnActorFromClass` "/Game/Yuqi/Blueprint/BP_SandCube.BP_SandCube_C" (`self.GetTransform`) "Undefined" "MultiplyWithRoot" null null))
    (set `self.AlreadyMouldActor` _returnvalue)
    (`self.Cube Move`)))

(event `Cube Move`
  (`KismetSystemLibrary.Delay` 1.0)
  (set `self.CurrentLocation` (`SceneComponent.RelativeLocation` (`self.TransparentCube`)))
  (bind (_direction _newtrack_0) (`Timeline|Timeline` :!label _label)
    (:`Update`
      (`SceneComponent.K2_SetRelativeLocation` (`self.TransparentCube`) (+ (`self.CurrentLocation`) (* (`KismetMathLibrary.GetForwardVector` (`self.K2_GetActorRotation`)) (* _newtrack_0 180.0))) false false))
    (:`Finished`
      (`|ExecutionSequence`
        (:`then_0`
          (goto _label :!via `Reverse`))
        (:`then_1`
          (`KismetSystemLibrary.Delay` 0.8)
          (set `self.canMouldCube?` true))))))

(fn `UserConstructionScript`)