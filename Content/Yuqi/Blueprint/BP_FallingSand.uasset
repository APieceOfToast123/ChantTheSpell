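; Falling sand actor that changes the vertical scale of five static meshes according to the state of a sand anchor.
; BeginPlay casts its child actor to BP_SandAnchor and stores the reference.
; Each Tick polls the anchor's CanBreak flag, setting the meshes' Z scale to the Height variable when true and restoring a fixed default scale otherwise.
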(event `self.ReceiveBeginPlay`
  (bind _asbp_sand_anchor (cast `/Game/Yuqi/Blueprint/BP_SandAnchor` (`ChildActorComponent.ChildActor` (`self.BP_SandAnchor`))))
  (set `self.Sand Anchor` _asbp_sand_anchor))

(event `self.ReceiveTick`
  (params (DeltaSeconds :type "Float (single-precision)"))
  (if (`/Game/Yuqi/Blueprint/BP_SandAnchor.canBreak?` (`self.Sand Anchor`))
    (`SceneComponent.SetRelativeScale3D` (`self.StaticMesh`) (`KismetMathLibrary.MakeVector` 2.0 5.0 (`self.Height`)))
    (`SceneComponent.SetRelativeScale3D` (`self.StaticMesh1`) (`KismetMathLibrary.MakeVector` 2.0 5.0 (`self.Height`)))
    (`SceneComponent.SetRelativeScale3D` (`self.StaticMesh2`) (`KismetMathLibrary.MakeVector` 2.0 5.0 (`self.Height`)))
    (`SceneComponent.SetRelativeScale3D` (`self.StaticMesh3`) (`KismetMathLibrary.MakeVector` 2.0 5.0 (`self.Height`)))
    (`SceneComponent.SetRelativeScale3D` (`self.StaticMesh4`) (`KismetMathLibrary.MakeVector` 2.0 5.0 (`self.Height`)))
    (else
      (`SceneComponent.SetRelativeScale3D` (`self.StaticMesh`) (2.0 5.0 2.0))
      (`SceneComponent.SetRelativeScale3D` (`self.StaticMesh1`) (2.0 5.0 2.0))
      (`SceneComponent.SetRelativeScale3D` (`self.StaticMesh2`) (2.0 5.0 2.0))
      (`SceneComponent.SetRelativeScale3D` (`self.StaticMesh3`) (2.0 5.0 2.0))
      (`SceneComponent.SetRelativeScale3D` (`self.StaticMesh4`) (2.0 5.0 2.0)))))

(fn `UserConstructionScript`)