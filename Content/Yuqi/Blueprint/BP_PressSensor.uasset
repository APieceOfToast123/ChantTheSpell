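; Pressure plate actor that responds to BP_ThirdPersonCharacter1 or actors tagged "Weight" entering its box.
; Pressing plays a success sound and runs a timeline that sinks the mesh along its local down axis, reversing when the last tracked occupant leaves.
; TrySpawnWind, not called within this graph, spawns a BP_CubeWind at the stored scene component location while pressed, or destroys it otherwise.
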(event `self.ReceiveBeginPlay`
  (set `self.SceneNodeLocation` (`SceneComponent.K2_GetComponentLocation` (`self.Scene`))))

(event `self.ReceiveTick`
  (params (DeltaSeconds :type "Float (single-precision)")))

(event `self.Box.OnComponentBeginOverlap`
  (params (OverlappedComponent :type "PrimitiveComponent Object Reference") (OtherActor :type "Actor Object Reference") (OtherComp :type "PrimitiveComponent Object Reference") (OtherBodyIndex :type Integer) (bFromSweep :type Boolean) (SweepResult :type "HitResult Structure (by ref)"))
  (if (`self.canOpen`)
    (if (not (`self.State_isOpen`))
      (bind _asbp_third_person_character_1 (cast `/Game/ThirdPerson/Blueprints/BP_ThirdPersonCharacter1` OtherActor)
        (:`then`
          (`KismetArrayLibrary.Array_Add` (`self.PressedObject`) _asbp_third_person_character_1)
          (`self.OnPressSensor` :!label _label))
        (:`CastFailed`
          (if (`self.ActorHasTag` OtherActor "Weight")
            (`KismetArrayLibrary.Array_Add` (`self.PressedObject`) OtherActor)
            (goto _label)))))))

(event `self.Box.OnComponentEndOverlap`
  (params (OverlappedComponent :type "PrimitiveComponent Object Reference") (OtherActor :type "Actor Object Reference") (OtherComp :type "PrimitiveComponent Object Reference") (OtherBodyIndex :type Integer))
  (if (`KismetArrayLibrary.Array_Contains` (`self.PressedObject`) OtherActor)
    (if (<= (`KismetArrayLibrary.Array_Length` (`self.PressedObject`)) 1)
      (set `self.State_isOpen` false)
      (set `self.canOpen` true)
      (`self.OnUnPressSensor`)
      (`KismetArrayLibrary.Array_RemoveItem` (`self.PressedObject`) OtherActor)
      (goto _label_2 :!via `Reset`))))

(event `OnPressSensor`
  (set `self.State_isOpen` true)
  (`GameplayStatics.PlaySound2D` "/Game/Qianlin/Asset/SFX_Success.SFX_Success" 1.0 1.0 0.0 null null)
  (`/Engine/EditorBlueprintResources/StandardMacros.DoOnce` false :!label _label_2
    (:`Completed`
      (set `self.currentSensorLocation` (`SceneComponent.RelativeLocation` (`self.StaticMesh`)))
      (bind (_direction _newtrack_0) (`Timeline|Timeline` :!label _label_3)
        (:`Update`
          (`SceneComponent.K2_SetRelativeLocation` (`self.StaticMesh`) (+ (`self.currentSensorLocation`) (* (`KismetMathLibrary.NegateVector` (`KismetMathLibrary.GetUpVector` (`self.K2_GetActorRotation`))) (* _newtrack_0 8.0))) false false))))))

(event `OnUnPressSensor`
  (goto _label_3 :!via `ReverseFromEnd`))

(event `Try Spawn Wind`
  (if (`self.State_isOpen`)
    (if (`self.canOpen`)
      (set `self.canOpen` false)
      (if (!= (`self.SceneNodeLocation`) (0.0 0.0 0.0) :`ErrorTolerance` 0.99)
        (bind _returnvalue (`|SpawnActorFromClass` "/Game/Yuqi/Blueprint/BP_CubeWind.BP_CubeWind_C" (`KismetMathLibrary.MakeTransform` (`self.SceneNodeLocation`)) "AlwaysSpawn" "MultiplyWithRoot" null 1800 800.0 400.0 null))
        (set `self.Cube Wind Tunnel` _returnvalue)))
    (elif (!= (`self.Cube Wind Tunnel`) null)
      (`self.K2_DestroyActor` (`self.Cube Wind Tunnel`))
      (set `self.Cube Wind Tunnel` null))))

(fn `UserConstructionScript`
  (`SceneComponent.K2_SetWorldLocation` (`self.Scene`) (`self.SceneNodeLocation`) false false))