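; Interactable valve that turns itself and an assigned WindAnchor actor, with an optional camera cut to show the result.
; A box overlap gates the interact input and shows a prompt widget that faces the follow camera.
; A FlipFlop alternates blending to a CameraActor matched by display name while freezing movement and rotating, then returning to the player.
; Timelines drive rotations on a selectable axis for the anchor; without a camera, every press rotates.
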(event `EnhancedInput|/Game/ThirdPerson/Input/Actions/IA_Interact`
  (params (ActionValue :type Boolean) (ElapsedSeconds :type "Float (double-precision)") (TriggeredSeconds :type "Float (double-precision)") (InputAction :type "InputAction Object Reference" :default "/Game/ThirdPerson/Input/Actions/IA_Interact.IA_Interact"))
  (:`Triggered`
    (`/Engine/EditorBlueprintResources/StandardMacros.Gate` true :!label _label
      (:`Exit`
        (`/Game/Dialogue/BPI_Dialogue.Talk`)))))

(event `self.ReceiveTick`
  (params (DeltaSeconds :type "Float (single-precision)"))
  (bind _widget (`self.Widget`)
    (:`then`
      (bind _asbp_third_person_character_1 (cast `/Game/ThirdPerson/Blueprints/BP_ThirdPersonCharacter1` (`GameplayStatics.GetPlayerCharacter` 0)))
      (`SceneComponent.K2_SetWorldRotation` _widget (`KismetMathLibrary.FindLookAtRotation` (`SceneComponent.K2_GetComponentLocation` _widget) (`SceneComponent.K2_GetComponentLocation` (`/Game/ThirdPerson/Blueprints/BP_ThirdPersonCharacter1.FollowCamera` _asbp_third_person_character_1))) false false))
    (:`else`)))

(event `self.Box.OnComponentBeginOverlap`
  (params (OverlappedComponent :type "PrimitiveComponent Object Reference") (OtherActor :type "Actor Object Reference") (OtherComp :type "PrimitiveComponent Object Reference") (OtherBodyIndex :type Integer) (bFromSweep :type Boolean) (SweepResult :type "HitResult Structure (by ref)"))
  (if (== OtherActor (`GameplayStatics.GetPlayerPawn` 0))
    (`TextBlock.SetOpacity` (`self.Text`) 1.0)
    (`self.EnableInput` (`GameplayStatics.GetPlayerController` 0))
    (goto _label :!via `Open`)))

(event `self.Box.OnComponentEndOverlap`
  (params (OverlappedComponent :type "PrimitiveComponent Object Reference") (OtherActor :type "Actor Object Reference") (OtherComp :type "PrimitiveComponent Object Reference") (OtherBodyIndex :type Integer))
  (`TextBlock.SetOpacity` (`self.Text`) 0.0)
  (goto _label :!via `Close`))

(event `self.ReceiveBeginPlay`
  (bind _aswb_press_to_do (cast `/Game/Yuqi/UI/WB_PressToDo` (`WidgetComponent.GetWidget` (`self.Widget`))))
  (bind _output_get (set `self.Text` (`/Game/Yuqi/UI/WB_PressToDo.Text` _aswb_press_to_do)))
  (`TextBlock.SetOpacity` _output_get 0.0))

(event `self.Talk`
  (`/Engine/EditorBlueprintResources/StandardMacros.FlipFlop`
    (:`A`
      (`self.Camera Come`)
      (`self.Rotate Valve` :!label _label_2)
      (`self.Rotate Wind Anchor`))
    (:`B`
      (if (not (`self.isCameraFound`))
        (goto _label_2)
        (else
          (`self.Camera Leave`))))))

(event `Rotate Valve`
  (bind (_valve_rotation_roll _valve_rotation_pitch) (`KismetMathLibrary.BreakRotator` (`self.Valve Rotation`)))
  (if (`self.canRotate`)
    (set `self.canRotate` false)
    (set `self.Valve Rotation` (`self.K2_GetActorRotation`))
    (`/Engine/EditorBlueprintResources/StandardMacros.DoOnce` false :!label _label_3
      (:`Completed`
        (`GameplayStatics.PlaySoundAtLocation` "/Game/BerkeleeSFX/Action/sfx_rotatevalve_v01.sfx_rotatevalve_v01" (`self.K2_GetActorLocation`) (struct) 1.0 1.0 0.0 null null null null)
        (bind (_direction _rotate_time) (`Timeline|Timeline_1` :!via `PlayFromStart`)
          (:`Update`
            (`SceneComponent.K2_SetRelativeRotation` (`self.StaticMesh`) (`KismetMathLibrary.MakeRotator` _valve_rotation_roll (+ _valve_rotation_pitch (`KismetMathLibrary.Lerp` 0.0 -50.0 _rotate_time))) false false))
          (:`Finished`
            (`KismetSystemLibrary.Delay` 0.75)
            (set `self.canRotate` true)
            (goto _label_3 :!via `Reset`)))))))

(event `Rotate Wind Anchor`
  (bind (_wind_anchor_rotation_roll _wind_anchor_rotation_pitch _wind_anchor_rotation_yaw) (`KismetMathLibrary.BreakRotator` (`self.Wind Anchor Rotation`)))
  (bind (_wind_anchor_rotation_roll_2 _wind_anchor_rotation_pitch_2 _wind_anchor_rotation_yaw_2) (`KismetMathLibrary.BreakRotator` (`self.Wind Anchor Rotation`)))
  (bind (_wind_anchor_rotation_roll_3 _wind_anchor_rotation_pitch_3 _wind_anchor_rotation_yaw_3) (`KismetMathLibrary.BreakRotator` (`self.Wind Anchor Rotation`)))
  (if (!= (`self.WindAnchor`) null)
    (set `self.Wind Anchor Rotation` (`SceneComponent.K2_GetComponentRotation` (`Actor.RootComponent` (`self.WindAnchor`))))
    (`/Engine/EditorBlueprintResources/StandardMacros.DoOnce` false :!label _label_4
      (:`Completed`
        (bind (_direction _rotate_time) (`Timeline|Timeline` :!via `PlayFromStart`)
          (:`Update`
            (switch `/Game/Yuqi/Blueprint/E_Rotation` (`self.Rotation Type`)
              (:`NewEnumerator0`
                (bind _returnvalue (`KismetMathLibrary.Lerp` 0.0 -90.0 _rotate_time))
                (`SceneComponent.K2_SetWorldRotation` (`Actor.RootComponent` (`self.WindAnchor`)) (`KismetMathLibrary.MakeRotator` (+ _returnvalue _wind_anchor_rotation_roll_3) _wind_anchor_rotation_pitch_3 _wind_anchor_rotation_yaw_3) false false))
              (:`NewEnumerator1`
                (`SceneComponent.K2_SetWorldRotation` (`Actor.RootComponent` (`self.WindAnchor`)) (`KismetMathLibrary.MakeRotator` _wind_anchor_rotation_roll_2 (+ _returnvalue _wind_anchor_rotation_pitch_2) _wind_anchor_rotation_yaw_2) false false))
              (:`NewEnumerator2`
                (`SceneComponent.K2_SetWorldRotation` (`Actor.RootComponent` (`self.WindAnchor`)) (`KismetMathLibrary.MakeRotator` _wind_anchor_rotation_roll _wind_anchor_rotation_pitch (+ _returnvalue _wind_anchor_rotation_yaw)) false false))))
          (:`Finished`
            (`KismetSystemLibrary.Delay` 0.75)
            (goto _label_4 :!via `Reset`)))))
    (else
      (`KismetSystemLibrary.PrintString` "Didn't set wind anchor"))))

(event `Camera Come`
  (bind _outactors (`GameplayStatics.GetAllActorsOfClass` "/Script/Engine.CameraActor"))
  (for _array_element _outactors
    (if (== (`KismetSystemLibrary.GetDisplayName` _array_element) (`self.CameraDisplayName`))
      (set `self.isCameraFound` true)
      (`PlayerController.SetViewTargetWithBlend` (`GameplayStatics.GetPlayerController` 0) _array_element (`self.Blend Time`) "VTBlend_Linear" 1.0 false)
      (`CharacterMovementComponent.SetMovementMode` (`Character.CharacterMovement` (`GameplayStatics.GetPlayerCharacter` 0)) "MOVE_None" 0)
      (`TextBlock.SetOpacity` (`self.Text`) 0.0)))
  (if (not (`self.isCameraFound`))
    _))

(event `Camera Leave`
  (`PlayerController.SetViewTargetWithBlend` (`GameplayStatics.GetPlayerController` 0) (`GameplayStatics.GetPlayerCharacter` 0) (`self.Blend Time`) "VTBlend_Linear" 0.0 false)
  (`CharacterMovementComponent.SetMovementMode` (`Character.CharacterMovement` (`GameplayStatics.GetPlayerCharacter` 0)) "MOVE_Walking" 0)
  (`KismetSystemLibrary.Delay` 0.5)
  (`TextBlock.SetOpacity` (`self.Text`) 1.0))

(fn `UserConstructionScript`)