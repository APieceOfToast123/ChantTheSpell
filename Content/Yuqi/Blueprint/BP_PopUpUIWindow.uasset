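; BP_PopUpUIWindow is a one-shot trigger actor that shows a pop-up message when a Player-tagged actor overlaps its Box.
; PopWindow disables Box collision, creates a WB_PopUpWindow with TextToShow and adds it to the viewport.
; A timeline fades in its opacity, with a delayed reverse called from the Update pin to fade it out.
; After a fixed delay from the overlap, RemoveWindow removes the widget and destroys the actor.
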(event `Pop Window`
  (bind _returnvalue (`|CreateWidget` "/Game/Yuqi/UI/WB_PopUpWindow.WB_PopUpWindow_C" (`GameplayStatics.GetPlayerController` 0)))
  (bind _output_get (set `self.PopWindowREF` _returnvalue))
  (`TextBlock.SetText` (`/Game/Yuqi/UI/WB_PopUpWindow.WindowText` _output_get) (`KismetTextLibrary.Conv_StringToText` (`self.TextToShow`)))
  (`PrimitiveComponent.SetCollisionEnabled` (`self.Box`) "NoCollision")
  (`UserWidget.AddToViewport` _output_get 0)
  (bind (_direction _newtrack_0) (`Timeline|Timeline` :!label _label)
    (:`Update`
      (`Widget.SetRenderOpacity` (`self.PopWindowREF`) _newtrack_0)
      (`KismetSystemLibrary.Delay` 3.0)
      (goto _label :!via `Reverse`))))

(event `RemoveWindow`
  (bind _popwindowref (`self.PopWindowREF`)
    (:`then`
      (`Widget.RemoveFromParent` _popwindowref)
      (`self.K2_DestroyActor`))
    (:`else`)))

(event `self.Box.OnComponentBeginOverlap`
  (params (OverlappedComponent :type "PrimitiveComponent Object Reference") (OtherActor :type "Actor Object Reference") (OtherComp :type "PrimitiveComponent Object Reference") (OtherBodyIndex :type Integer) (bFromSweep :type Boolean) (SweepResult :type "HitResult Structure (by ref)"))
  (if (`self.ActorHasTag` OtherActor "Player")
    (`self.Pop Window`)
    (`KismetSystemLibrary.Delay` 6.0)
    (`self.RemoveWindow`)))

(fn `UserConstructionScript`)