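; BP_MusicTrigger is a placed trigger that switches the background music when the player character enters its box.
; On the first overlap by BP_ThirdPersonCharacter1, it finds every BP_MusicTrigger in the level and fades out their stored sound instances.
; It then spawns its MusicREF as a 2D sound, stores the instance and fades it in, crossfading between tracks.
; A DoOnce with no reset limits each trigger to a single activation.
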(event `self.Box.OnComponentBeginOverlap`
  (params (OverlappedComponent :type "PrimitiveComponent Object Reference") (OtherActor :type "Actor Object Reference") (OtherComp :type "PrimitiveComponent Object Reference") (OtherBodyIndex :type Integer) (bFromSweep :type Boolean) (SweepResult :type "HitResult Structure (by ref)"))
  (cast `/Game/ThirdPerson/Blueprints/BP_ThirdPersonCharacter1` OtherActor)
  (`/Engine/EditorBlueprintResources/StandardMacros.DoOnce` false
    (:`Completed`
      (bind _outactors (`GameplayStatics.GetAllActorsOfClass` "BP_MusicTrigger_C"))
      (for _array_element _outactors
        (bind _soundinstance (`/Game/Yuqi/Blueprint/BP_MusicTrigger.SoundInstance` _array_element))
        (if (!= _soundinstance null)
          (`AudioComponent.FadeOut` _soundinstance 0.3 0.0 "Linear")))
      (bind _returnvalue (`GameplayStatics.SpawnSound2D` (`self.Music REF`) 1.0 1.0 0.0 null))
      (set `self.SoundInstance` _returnvalue)
      (`AudioComponent.FadeIn` _returnvalue 0.5 1.0 0.0 "Linear"))))

(fn `UserConstructionScript`)