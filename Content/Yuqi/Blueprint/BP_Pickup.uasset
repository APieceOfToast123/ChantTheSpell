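; Collectible rune pickup that the player collects with the Interact action, announced by a floating "Press B to Collect Rune" prompt.
; Player overlap with the Box enables input and opens a gate, and nothing closes it on leaving.
; Interacting fires the OnPickUp dispatcher, plays a sound and destroys the actor a tick later.
; Tick rotates the prompt widget to face the third-person character's follow camera.
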(event `EnhancedInput|/Game/ThirdPerson/Input/Actions/IA_Interact`
  (params (ActionValue :type Boolean) (ElapsedSeconds :type "Float (double-precision)") (TriggeredSeconds :type "Float (double-precision)") (InputAction :type "InputAction Object Reference" :default "/Game/ThirdPerson/Input/Actions/IA_Interact.IA_Interact"))
  (:`Triggered`
    (`/Engine/EditorBlueprintResources/StandardMacros.Gate` true :!label _label
      (:`Exit`
        (`self.OnPickUp`)
        (`GameplayStatics.PlaySound2D` "/Game/BerkeleeSFX/Arriaga_Isabel_CTS_sfx_action_runeadquire_v02.Arriaga_Isabel_CTS_sfx_action_runeadquire_v02" 1.0 1.0 0.0 null null false)
        (`KismetSystemLibrary.DelayUntilNextTick`)
        (`self.K2_DestroyActor`)))))

(event `self.Box.OnComponentBeginOverlap`
  (params (OverlappedComponent :type "PrimitiveComponent Object Reference") (OtherActor :type "Actor Object Reference") (OtherComp :type "PrimitiveComponent Object Reference") (OtherBodyIndex :type Integer) (bFromSweep :type Boolean) (SweepResult :type "HitResult Structure (by ref)"))
  (if (== OtherActor (`GameplayStatics.GetPlayerPawn` 0))
    (`self.EnableInput` (`GameplayStatics.GetPlayerController` 0))
    (goto _label :!via `Open`)))

(event `self.ReceiveTick`
  (params (DeltaSeconds :type "Float (single-precision)"))
  (bind _widget (`self.Widget`)
    (:`then`
      (bind _asbp_third_person_character_1 (cast `/Game/ThirdPerson/Blueprints/BP_ThirdPersonCharacter1` (`GameplayStatics.GetPlayerCharacter` 0)))
      (`SceneComponent.K2_SetWorldRotation` _widget (`KismetMathLibrary.FindLookAtRotation` (`SceneComponent.K2_GetComponentLocation` _widget) (`SceneComponent.K2_GetComponentLocation` (`/Game/ThirdPerson/Blueprints/BP_ThirdPersonCharacter1.FollowCamera` _asbp_third_person_character_1))) false false))
    (:`else`)))

(event `self.ReceiveBeginPlay`
  (bind _aswb_press_to_do (cast `/Game/Yuqi/UI/WB_PressToDo` (`WidgetComponent.GetWidget` (`self.Widget`))))
  (set `TextBlock.Text` "Press B to Collect Rune" (`/Game/Yuqi/UI/WB_PressToDo.Text` _aswb_press_to_do)))

(fn `UserConstructionScript`)