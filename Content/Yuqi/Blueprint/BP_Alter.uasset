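; Altar actor that tracks pickups left to collect in its area and is solved once none remain.
; Each pickup's OnPickUp decrements the remaining count.
; Inside the trigger box, Interact toggles between blending to a display-name-matched CameraActor with player movement disabled, and returning to the character.
; Interacting in also shows the hint widget, updates its count if any were collected, and broadcasts OnAltarSolved at zero.
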(event `self.ReceiveBeginPlay`
  (bind _pickupactorsinarea (`self.PickupActorsInArea`))
  (bind _returnvalue (`KismetTextLibrary.Conv_IntToText` (`self.LeftPickup`)))
  (set `self.LeftPickup` (`KismetArrayLibrary.Array_Length` _pickupactorsinarea))
  (for _array_element _pickupactorsinarea
    (add `/Game/Yuqi/Blueprint/BP_Pickup.OnPickUp` _array_element (delegate `UpdatePickupList`))
    (bind _aswb_alter_hint (cast `/Game/Yuqi/UI/WB_AlterHint` (`WidgetComponent.GetWidget` (`self.AlterHint`))))
    (`TextBlock.SetText` (`/Game/Yuqi/UI/WB_AlterHint.TotalPickup` _aswb_alter_hint) _returnvalue)
    (`TextBlock.SetText` (`/Game/Yuqi/UI/WB_AlterHint.LeftPickup` _aswb_alter_hint) _returnvalue)))

(event `UpdatePickupList`
  (bind _result (`/Engine/EditorBlueprintResources/StandardMacros.DecrementInt` (`self.LeftPickup`))
    (:`  `
      (set `self.LeftPickup` _result))))

(event `EnhancedInput|/Game/ThirdPerson/Input/Actions/IA_Interact`
  (params (ActionValue :type Boolean) (ElapsedSeconds :type "Float (double-precision)") (TriggeredSeconds :type "Float (double-precision)") (InputAction :type "InputAction Object Reference" :default "/Game/ThirdPerson/Input/Actions/IA_Interact.IA_Interact"))
  (:`Triggered`
    (`/Engine/EditorBlueprintResources/StandardMacros.Gate` true :!label _label
      (:`Exit`
        (`/Engine/EditorBlueprintResources/StandardMacros.FlipFlop`
          (:`A`
            (`SceneComponent.SetVisibility` (`self.PressToDo`) false false)
            (`SceneComponent.SetVisibility` (`self.AlterHint`) true false)
            (`self.Check Pickup`)
            (`self.CameraMove`))
          (:`B`
            (`self.CameraBack`)))))))

(event `self.Box.OnComponentBeginOverlap`
  (params (OverlappedComponent :type "PrimitiveComponent Object Reference") (OtherActor :type "Actor Object Reference") (OtherComp :type "PrimitiveComponent Object Reference") (OtherBodyIndex :type Integer) (bFromSweep :type Boolean) (SweepResult :type "HitResult Structure (by ref)"))
  (if (not (`self.isAltarSolved?`))
    (`SceneComponent.SetVisibility` (`self.PressToDo`) true false)
    (`self.EnableInput` (`GameplayStatics.GetPlayerController` 0))
    (goto _label :!via `Open`)))

(event `self.Box.OnComponentEndOverlap`
  (params (OverlappedComponent :type "PrimitiveComponent Object Reference") (OtherActor :type "Actor Object Reference") (OtherComp :type "PrimitiveComponent Object Reference") (OtherBodyIndex :type Integer))
  (if (not (`self.isAltarSolved?`))
    (`SceneComponent.SetVisibility` (`self.PressToDo`) false false)
    (`SceneComponent.SetVisibility` (`self.AlterHint`) false false)
    (goto _label :!via `Close`)))

(event `Check Pickup`
  (if (`self.isAltarSolved?`)
    _
    (elif (not (== (`KismetArrayLibrary.Array_Length` (`self.PickupActorsInArea`)) (`self.LeftPickup`)))
      (bind _aswb_alter_hint (cast `/Game/Yuqi/UI/WB_AlterHint` (`WidgetComponent.GetWidget` (`self.AlterHint`))))
      (`TextBlock.SetText` (`/Game/Yuqi/UI/WB_AlterHint.LeftPickup` _aswb_alter_hint) (`KismetTextLibrary.Conv_IntToText` (`self.LeftPickup`)))
      (`GameplayStatics.PlaySound2D` "/Game/Qianlin/Asset/SFX_Success.SFX_Success" 1.0 1.0 0.0 null null)
      (if (== (`self.LeftPickup`) 0)
        (set `self.isAltarSolved?` true)
        (`KismetSystemLibrary.Delay` 0.2)
        (`self.OnAltarSolved`)
        (goto _label :!via `Close`)))))

(event `CameraMove`
  (bind _outactors (`GameplayStatics.GetAllActorsOfClass` "/Script/Engine.CameraActor"))
  (for _array_element _outactors
    (if (== (`KismetSystemLibrary.GetDisplayName` _array_element) (`self.Camera Display Name`))
      (set `self.Is Camera Found` true)
      (`PlayerController.SetViewTargetWithBlend` (`GameplayStatics.GetPlayerController` 0) _array_element (`self.Blend Time`) "VTBlend_Linear" 1.0 false)
      (`CharacterMovementComponent.SetMovementMode` (`Character.CharacterMovement` (`GameplayStatics.GetPlayerCharacter` 0)) "MOVE_None" 0)))
  (if (not (`self.Is Camera Found`))
    (`KismetSystemLibrary.PrintString` "Didn't Set Camera")))

(event `CameraBack`
  (`PlayerController.SetViewTargetWithBlend` (`GameplayStatics.GetPlayerController` 0) (`GameplayStatics.GetPlayerCharacter` 0) (`self.Blend Time`) "VTBlend_Linear" 0.5 false)
  (`CharacterMovementComponent.SetMovementMode` (`Character.CharacterMovement` (`GameplayStatics.GetPlayerCharacter` 0)) "MOVE_Walking" 0))

(fn `UserConstructionScript`)