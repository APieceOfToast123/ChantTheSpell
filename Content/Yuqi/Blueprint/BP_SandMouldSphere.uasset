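; Sand mould station that produces a BP_SandSphere, with a prompt widget that turns to face the player's follow camera.
; The Moulding event, gated by CanMouldSphere, destroys the previous sphere, plays Niagara and sound effects, then spawns a new one after a delay.
; A Timeline then slides TransparentCube out along its relative X axis and reverses it, with moulding re-enabled shortly after.
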(event `self.ReceiveTick`
  (params (DeltaSeconds :type "Float (single-precision)"))
  (bind _widget (`self.Widget`))
  (bind _asbp_third_person_character_1 (cast `/Game/ThirdPerson/Blueprints/BP_ThirdPersonCharacter1` (`GameplayStatics.GetPlayerCharacter` 0)))
  (`SceneComponent.K2_SetWorldRotation` _widget (`KismetMathLibrary.FindLookAtRotation` (`SceneComponent.K2_GetComponentLocation` _widget) (`SceneComponent.K2_GetComponentLocation` (`/Game/ThirdPerson/Blueprints/BP_ThirdPersonCharacter1.FollowCamera` _asbp_third_person_character_1))) false false))

(event `self.ReceiveBeginPlay`
  (bind _aswb_press_to_do (cast `/Game/Yuqi/UI/WB_PressToDo` (`WidgetComponent.GetWidget` (`self.Widget`))))
  (set `TextBlock.Text` "Press LT and click B to generate sand mould" (`/Game/Yuqi/UI/WB_PressToDo.Text` _aswb_press_to_do)))

(event `Moulding`
  (if (`self.canMouldSphere?`)
    (set `self.canMouldSphere?` false)
    (if (!= (`self.AlreadyMouldActor`) null)
      (`self.K2_DestroyActor` (`self.AlreadyMouldActor`)))
    (`ActorComponent.Activate` (`self.Niagara`) false)
    (`GameplayStatics.PlaySound2D` "/Game/Qianlin/Asset/SFX_Success.SFX_Success" 1.0 1.0 0.0 null null)
    (`KismetSystemLibrary.Delay` 5.0)
    (bind _returnvalue (`|SpawnActorFromClass` "/Game/Yuqi/Blueprint/BP_SandSphere.BP_SandSphere_C" (`self.GetTransform`) "Undefined" "MultiplyWithRoot" null null))
    (set `self.AlreadyMouldActor` _returnvalue)
    (`self.Move`)))

(event `Move`
  (`KismetSystemLibrary.Delay` 1.0)
  (set `self.CurrentLocation` (`SceneComponent.RelativeLocation` (`self.TransparentCube`)))
  (bind (_direction _newtrack_0) (`Timeline|Timeline` :!label _label)
    (:`Update`
      (`SceneComponent.K2_SetRelativeLocation` (`self.TransparentCube`) (+ (`self.CurrentLocation`) (* (`KismetMathLibrary.Vector_Forward`) (* _newtrack_0 180.0))) false false))
    (:`Finished`
      (`|ExecutionSequence`
        (:`then_0`
          (goto _label :!via `Reverse`))
        (:`then_1`
          (`KismetSystemLibrary.Delay` 0.8)
          (set `self.canMouldSphere?` true))))))

(fn `UserConstructionScript`)